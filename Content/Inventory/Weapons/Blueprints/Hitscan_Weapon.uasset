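; Hitscan weapon Blueprint that, on Fire, traces on Visibility from just above the muzzle socket to a far point along the owner's eye view.
; Muzzle effects, sound and tracer play before the trace, so the tracer targets the previously saved hit point.
; The hit's physical surface is saved; only Vulnerable hits on a PlayerPawn apply damage and reach PlayHitEffects, which selects flesh or surface effects.
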(event EventBeginPlay
  (|CallParentFunction) ; This node is disabled and will not be called.\nDrag off pins to build functionality.
)

(event Collision|EventActorBeginOverlap
  (params (OtherActor :type Actor%20Object%20Reference))
  (|CallParentFunction OtherActor) ; This node is disabled and will not be called.\nDrag off pins to build functionality.
)

(event EventTick
  (params (DeltaSeconds :type Float%20%28single-precision%29))
  (|CallParentFunction DeltaSeconds) ; This node is disabled and will not be called.\nDrag off pins to build functionality.
)

(event EventFire
  (CallFunction|HitscanFire))

(fn ConstructionScript
  (|CallParentFunction))

(fn HitscanFire
  (CallFunction|PlayFireEffects)
  (bind _outhit (Collision|LineTraceByChannel (Utilities|GetMuzzleLocation) (Utilities|GetTraceEnd) "TraceTypeQuery1" false 0 "None"))
  (bind _surfacetypeout (Utilities|SaveHitVariables (.impactpoint _outhit) (.physmat _outhit))
    (:ExecPinOut
      (switch Utilities|FlowControl|Switch|SwitchonEPhysicalSurface _surfacetypeout
        (:SurfaceType1
          (bind _asplayer_pawn (Utilities|Casting|CastToPlayerPawn (.hitactor _outhit)))
          (bind _output_get (Variables|Default|SetPlayerHit _asplayer_pawn))
          (bind _newparam (Utilities|GetOwnerController)
            (:ExecPinOut
              (Game|Damage|ApplyDamage _output_get (Variables|Default|GetWeaponDamage) _newparam self "/Script/Engine.DamageType")
              (CallFunction|PlayHitEffects))))))))

(fn PlayHitEffects
  (bind _hiteffectssurface (Variables|Default|GetHitEffectsSurface))
  (bind _hiteffectsflesh (Variables|Default|GetHitEffectsFlesh))
  (switch Utilities|FlowControl|Switch|SwitchonEPhysicalSurface (Variables|Default|GetHitSurfaceType)
    (:SurfaceType_Default
      (Utilities|SpawnHitEffects (.soundeffect _hiteffectssurface) (.visualeffect _hiteffectssurface)))
    (:SurfaceType1
      (Utilities|SpawnHitEffects (.soundeffect _hiteffectsflesh) (.visualeffect _hiteffectsflesh)))))

(fn PlayFireEffects
  (Effects|SpawnEmitterAttached (.visualeffect (Variables|Default|GetFireEffects)) (Variables|Default|GetWeaponMesh) (Variables|Default|GetMuzzleSocketName))
  (Audio|PlaySoundatLocation (.soundeffect (Variables|Default|GetFireEffects)) (Utilities|GetMuzzleLocation) "0, 0, 0" 0.3 1.0 0.0 0 0 0)
  (bind _returnvalue (Effects|SpawnEmitteratLocation (.visualeffect (Variables|Default|GetTracerEffects)) (Utilities|GetMuzzleLocation)))
  (Effects|Components|ParticleSystem|SetVectorParameter _returnvalue (Variables|Default|GetTracerTargetName) (Variables|Default|GetHitPoint)))